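; Level 5 actor that plays a scripted chromosome separation animation, then shows a cell body with an animated tail moving away.
; BeginPlay starts three slowed skeletal animations, one of them looping, and after a timed delay hides the separation mesh and reveals the body and tail meshes.
; The tail loops its animation while MoveComponentTo repositions CcBody2, then Tick pushes that body along its negative up vector by a fixed, frame-rate-dependent step.
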(event EventBeginPlay
  (bind _saperate (Variables|Default|Getsaperate))
  (bind _chromosome_sep_2 (Variables|Default|Getchromosome_sep_2))
  (bind _chromosome_sep_1 (Variables|Default|Getchromosome_sep_1))
  (Utilities|FlowControl|Sequence
    (:then_0
      (Components|Animation|PlayAnimation _saperate "/Game/Models/level05/cell_sap/saperate_ani.saperate_ani" false)
      (Components|Timeline|SetPlayRate _saperate 0.3))
    (:then_1
      (Components|Animation|PlayAnimation _chromosome_sep_2 "/Game/Models/level05/chro/chromosome_sep_2_ani.chromosome_sep_2_ani" true)
      (Components|Timeline|SetPlayRate _chromosome_sep_2 0.3))
    (:then_2
      (Components|Animation|PlayAnimation _chromosome_sep_1 "/Game/Models/level05/chro/chromosome_sep_1_ani.chromosome_sep_1_ani" false)
      (Components|Timeline|SetPlayRate _chromosome_sep_1 0.3)
      (Utilities|FlowControl|Delay 17.5)
      (Rendering|SetVisibility (Variables|Default|Getsaperate) false false)
      (Rendering|SetVisibility (Variables|Default|Getcc_body2) true false)
      (Rendering|SetVisibility (Variables|Default|GetCC_body) true false)
      (Rendering|SetVisibility (Variables|Default|GetCC_tail) true false)
      (Components|Animation|PlayAnimation (Variables|Default|GetCC_tail) "/Game/Models/cc_tail/CC_tail_ani.CC_tail_ani" true)
      (Components|MoveComponentTo (Variables|Default|Getcc_body2) "0.000000,0.000000,10.000000" "-90.000000, 0, 0" false false 4.0 false)
      (Variables|Default|Setis_move true))))

(event EventTick
  (params (DeltaSeconds :type Float%20%28single-precision%29))
  (bind _cc_body2 (Variables|Default|Getcc_body2))
  (if (Variables|Default|Getis_move)
    (Transformation|AddWorldOffset _cc_body2 (* (Math|Vector|NegateVector (Math|Vector|GetUpVector _cc_body2)) 0.5) false false)))

(fn ConstructionScript)