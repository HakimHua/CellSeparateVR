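; Level 4 Blueprint that plays a scripted molecular animation of Plactnome, Oric, and paired ParA and ATP models.
; BeginPlay starts every animation, looping only Plactnome, with a shared Rate for all but the slower Oric.
; A delay chain then shows and later hides the ParA and Atp components in staggered order.
; Tick keeps those two components floating just above sockets on the animated ParA02 and ATP01 meshes.
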(event EventBeginPlay
  (bind _plactnome (Variables|Default|Getplactnome))
  (bind _para01 (Variables|Default|GetParA01))
  (bind _para (Variables|Default|GetParA))
  (bind _atp (Variables|Default|Getatp))
  (bind _rate (Variables|Default|Getrate))
  (bind _para02 (Variables|Default|GetParA02))
  (bind _atp01 (Variables|Default|GetATP01))
  (bind _atp02 (Variables|Default|GetATP02))
  (bind _oric (Variables|Default|Getoric))
  (Utilities|FlowControl|Sequence
    (:then_0
      (Components|Animation|PlayAnimation _plactnome "/Game/Models/Level04/plactnome/plactnome_ani.plactnome_ani" true)
      (Components|Timeline|SetPlayRate _plactnome _rate))
    (:then_1
      (Components|Animation|PlayAnimation _para01 "/Game/Models/Level04/ParA_ani/ParA01_Anim.ParA01_Anim" false)
      (Components|Timeline|SetPlayRate _para01 _rate))
    (:then_2
      (Components|Animation|PlayAnimation _para02 "/Game/Models/Level04/ParA_ani/ParA02_Anim.ParA02_Anim" false)
      (Components|Timeline|SetPlayRate _para02 _rate))
    (:then_3
      (Components|Animation|PlayAnimation _atp01 "/Game/Models/Level04/ParA_ani/ATP01_Anim.ATP01_Anim" false)
      (Components|Timeline|SetPlayRate _atp01 _rate))
    (:then_4
      (Components|Animation|PlayAnimation _atp02 "/Game/Models/Level04/ParA_ani/ATP02_Anim.ATP02_Anim" false)
      (Components|Timeline|SetPlayRate _atp02 _rate))
    (:then_5
      (Components|Animation|PlayAnimation _oric "/Game/Models/Level04/oric/oric_ani.oric_ani" false)
      (Components|Timeline|SetPlayRate _oric 0.2)
      (Utilities|FlowControl|Delay 2e+01)
      (Rendering|SetVisibility _para true false)
      (Utilities|FlowControl|Delay 2.0)
      (Rendering|SetVisibility _atp true false)
      (Utilities|FlowControl|Delay 8.0)
      (Rendering|SetVisibility _para false false)
      (Utilities|FlowControl|Delay 2.0)
      (Rendering|SetVisibility _atp false false))))

(event EventTick
  (params (DeltaSeconds :type Float%20%28single-precision%29))
  (Transformation|SetWorldLocation (Variables|Default|GetParA) (+ (Transformation|GetSocketLocation (Variables|Default|GetParA02) "ParA002") "0, 0,30.000000") false false)
  (Transformation|SetWorldLocation (Variables|Default|Getatp) (+ (Transformation|GetSocketLocation (Variables|Default|GetATP01) "ATP01") "0, 0,30.000000") false false))

(fn ConstructionScript)